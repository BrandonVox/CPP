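; BP_TraceActor is a debug tracing actor that shows what lies along its forward vector.
; Every Tick it runs a multi line trace for a single object type, with the end point computed from location, direction and length.
; For each hit it prints the bone name and draws a debug sphere at the impact point, alongside the one-frame trace line.
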(event EventTick
  (params (DeltaSeconds :type Float%20%28single-precision%29))
  (bind _returnvalue (Transformation|GetActorLocation))
  (bind _outhits (Class|KismetSystemLibrary|LineTraceMultiforObjects _returnvalue (|(A+(Direction*TraceLength)) _returnvalue 1e+03 (Transformation|GetActorForwardVector)) (Utilities|Array|MakeArray "ObjectTypeQuery7") false 0 "ForOneFrame" true))
  (for _array_element _outhits
    (Development|PrintString (Utilities|String|ToString(Name) (.HitBoneName (Collision|BreakHitResult _array_element))) true true "(R=0.000000,G=0.660000,B=1.000000,A=1.000000)" 1.0)
    (Rendering|Debug|DrawDebugSphere (.ImpactPoint (Collision|BreakHitResult _array_element)) 1e+01 12 "(R=1.000000,G=1.000000,B=1.000000,A=1.000000)" 0.0 2.0)))

(fn ConstructionScript)